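; BP_RoomNodeActor is a clickable map node actor representing a Monster, Elite, Shop or Event room.
; On BeginPlay, ShowWidget writes the Roomtype name into its WBP_MapData widget component and makes it visible.
; Clicking the mesh only prints a message for that room type.
; HideWidget can collapse the label, but the cursor-over bindings are never executed and SetMaterial is an empty stub.
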(event OnClicked(StaticMesh)
  (params (TouchedComponent :type Primitive%20Component%20Object%20Reference) (ButtonPressed :type Key%20Structure :default "None"))
  (switch Utilities|FlowControl|Switch|SwitchonEN_MapDataTypes (Variables|Default|GetRoomtype)
    (:NewEnumerator1
      (Development|PrintString "This is Battle Node!" true true "(R=0.000000,G=0.660000,B=1.000000,A=1.000000)" 1e+01))
    (:NewEnumerator2
      (Development|PrintString "This is Super Enemy Battle Node!" true true "(R=0.000000,G=0.660000,B=1.000000,A=1.000000)" 1e+01))
    (:NewEnumerator3
      (Development|PrintString "This is Shop Node!" true true "(R=0.000000,G=0.660000,B=1.000000,A=1.000000)" 1e+01))
    (:NewEnumerator5
      (Development|PrintString "This is Event Node!" true true "(R=0.000000,G=0.660000,B=1.000000,A=1.000000)" 1e+01))))

(event EventBeginPlay
  (CallFunction|ShowWidget))

(fn ConstructionScript)

(fn ShowWidget
  (params (TouchedComponent :type Primitive%20Component%20Object%20Reference))
  (bind _aswbp_map_data (Utilities|Casting|CastToWBP_MapData (UserInterface|GetUserWidgetObject (Variables|Default|GetMapWidgetComponent))))
  (Default|SetName _aswbp_map_data (Utilities|String|EnumtoString (Variables|Default|GetRoomtype)))
  (Widget|SetVisibility _aswbp_map_data "Visible"))

(fn HideWidget
  (params (TouchedActor :type Actor%20Object%20Reference))
  (bind _aswbp_map_data (Utilities|Casting|CastToWBP_MapData (UserInterface|GetUserWidgetObject (Variables|Default|GetMapWidgetComponent))))
  (Variables|/Script/UMG.Widget|SetVisibility _aswbp_map_data "Collapsed"))

(fn SetMaterial
  (params (Number :type Integer)))